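; A scratch test Blueprint with character movement and capsule components, whose only live behavior prints the CharacterMovement velocity when K is pressed.
; Tick and the construction script are empty.
; Disconnected leftover nodes cover a Sensors_BP lookup and overlap check, copying the capsule's world location into myGameInstance's MainActorLocation, and debug prints, none of which execute.
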(event `Key|K`
  (params (Key :type "Key Structure"))
  (:`Pressed`
    (`KismetSystemLibrary.PrintString` (`KismetStringLibrary.Conv_VectorToString` (`MovementComponent.Velocity` (`self.CharacterMovement`))) true false)))

(event `self.ReceiveTick`
  (params (DeltaSeconds :type "Float (single-precision)")))

(fn `UserConstructionScript`)